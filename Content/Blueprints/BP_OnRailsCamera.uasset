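; BP_OnRailsCamera is a rail-mounted cine camera that becomes the first player's view when play begins.
; On BeginPlay it finds the first OnRailsCharacter2_5D and sets the CineCamera to tracking focus on that actor.
; It then places the camera once on RailSplineComponent, at the point closest to an unset world location input.
; Tick is disabled, so this graph never moves the camera along the rail afterward.
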(event EventBeginPlay
  (bind _cinecamera (Variables|Default|GetCineCamera))
  (Game|Player|SetViewTargetwithBlend (Game|GetPlayerController 0) self 0.0 "VTBlend_Linear" 0.0 false)
  (bind _outactors (Actor|GetAllActorsOfClass "/Script/Platformer2D3D.OnRailsCharacter2_5D"))
  (Variables|/Script/CinematicCamera.CineCameraComponent|SetFocusSettings _cinecamera (Utilities|Struct|MakeCameraFocusSettings "Tracking" (.manualfocusdistance (Variables|/Script/CinematicCamera.CineCameraComponent|GetFocusSettings _cinecamera)) (Utilities|Struct|MakeCameraTrackingFocusSettings (Utilities|ResolveSoftReference (Utilities|Array|Get(acopy) _outactors)) (.relativeoffset (.trackingfocussettings (Variables|/Script/CinematicCamera.CineCameraComponent|GetFocusSettings _cinecamera))) (.bdrawdebugtrackingfocuspoint (.trackingfocussettings (Variables|/Script/CinematicCamera.CineCameraComponent|GetFocusSettings _cinecamera)))) (.bsmoothfocuschanges (Variables|/Script/CinematicCamera.CineCameraComponent|GetFocusSettings _cinecamera)) (.focussmoothinginterpspeed (Variables|/Script/CinematicCamera.CineCameraComponent|GetFocusSettings _cinecamera)) (.focusoffset (Variables|/Script/CinematicCamera.CineCameraComponent|GetFocusSettings _cinecamera))))
  (Transformation|SetWorldLocation (Variables|Default|GetCineCamera) (Spline|FindLocationClosesttoWorldLocation (Variables|Default|GetRailSplineComponent) "0, 0, 0" "World") false false))

(event Collision|EventActorBeginOverlap
  (params (OtherActor :type Actor%20Object%20Reference)))

(event EventTick
  (params (DeltaSeconds :type Float%20%28single-precision%29)))

(fn ConstructionScript)