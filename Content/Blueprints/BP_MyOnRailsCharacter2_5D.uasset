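; On-rails 2.5D character that animates as a sprite-sheet flipbook through a dynamic material created on its mesh in the construction script.
; Spline move and jump input, falling, jump apex and landing each look up a state in AnimationStateMappings and push its sheet, rows and columns to the material.
; Move input also sets facing, and the apex shows a brief transition before Falling.
; The JumpTimer setup feeding AnimTimer is disconnected.
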(event Custom|JumpTimer
  (Rendering|Material|SetScalarParameterValue (Variables|Default|GetcharMat) "AnimTimer" (Class|KismetSystemLibrary|GetTimerElapsedTimeHandle (Variables|Default|GetJumpTimerHandle)) :!class /Script/Engine.MaterialInstanceDynamic))

(event Custom|JumpApexReached
  (bind _charmat (Variables|Default|GetcharMat))
  (bind _animationstatemappings (Variables|Default|GetAnimationStateMappings))
  (bind (_value _returnvalue) (Utilities|Map|Find _animationstatemappings "AirTrans"))
  (if _returnvalue
    (Rendering|Material|SetScalarParameterValue _charmat "UseAnimTimer" 1.0 :!class /Script/Engine.MaterialInstanceDynamic)
    (Rendering|Material|SetTextureParameterValue _charmat "Sprite" (.spritesheet _value))
    (Rendering|Material|SetScalarParameterValue _charmat "SpriteRows" (Math|Conversions|ToFloat(Integer) (.rows _value)) :!class /Script/Engine.MaterialInstanceDynamic)
    (Rendering|Material|SetScalarParameterValue _charmat "SpriteColumns" (Math|Conversions|ToFloat(Integer) (.columns _value)) :!class /Script/Engine.MaterialInstanceDynamic)
    (Utilities|FlowControl|Delay 0.2)
    (CallFunction|Falling)))

(event Custom|Falling
  (bind _charmat (Variables|Default|GetcharMat))
  (bind _animationstatemappings (Variables|Default|GetAnimationStateMappings))
  (bind (_value _returnvalue) (Utilities|Map|Find _animationstatemappings "Falling"))
  (if _returnvalue
    (Rendering|Material|SetScalarParameterValue _charmat "UseAnimTimer" 1.0 :!class /Script/Engine.MaterialInstanceDynamic)
    (Rendering|Material|SetTextureParameterValue _charmat "Sprite" (.spritesheet _value))
    (Rendering|Material|SetScalarParameterValue _charmat "SpriteRows" (Math|Conversions|ToFloat(Integer) (.rows _value)) :!class /Script/Engine.MaterialInstanceDynamic)
    (Rendering|Material|SetScalarParameterValue _charmat "SpriteColumns" (Math|Conversions|ToFloat(Integer) (.columns _value)) :!class /Script/Engine.MaterialInstanceDynamic)))

(event Custom|Idle
  (bind _charmat (Variables|Default|GetcharMat))
  (bind _animationstatemappings (Variables|Default|GetAnimationStateMappings))
  (bind (_value _returnvalue) (Utilities|Map|Find _animationstatemappings "Idle"))
  (if _returnvalue
    (Rendering|Material|SetTextureParameterValue _charmat "Sprite" (.spritesheet _value))
    (Rendering|Material|SetScalarParameterValue _charmat "SpriteRows" (Math|Conversions|ToFloat(Integer) (.rows _value)) :!class /Script/Engine.MaterialInstanceDynamic)
    (Rendering|Material|SetScalarParameterValue _charmat "SpriteColumns" (Math|Conversions|ToFloat(Integer) (.columns _value)) :!class /Script/Engine.MaterialInstanceDynamic)
    (Rendering|Material|SetScalarParameterValue _charmat "UseAnimTimer" 0.0 :!class /Script/Engine.MaterialInstanceDynamic)))

(event Input|EnhancedActionEvents|EnhancedInputActionIA_SplineMove
  (params (ActionValue :type Float%20%28double-precision%29) (ElapsedSeconds :type Float%20%28double-precision%29) (TriggeredSeconds :type Float%20%28double-precision%29) (InputAction :type Input%20Action%20Object%20Reference :default "/Game/Blueprints/Inputs/IA_SplineMove.IA_SplineMove"))
  (bind _charmat (Variables|Default|GetcharMat))
  (bind _animationstatemappings (Variables|Default|GetAnimationStateMappings))
  (bind (_value _returnvalue) (Utilities|Map|Find _animationstatemappings "Walk"))
  (:Triggered
    (if _returnvalue
      (Rendering|Material|SetTextureParameterValue _charmat "Sprite" (.spritesheet _value))
      (Rendering|Material|SetScalarParameterValue _charmat "SpriteRows" (Math|Conversions|ToFloat(Integer) (.rows _value)) :!class /Script/Engine.MaterialInstanceDynamic)
      (Rendering|Material|SetScalarParameterValue _charmat "SpriteColumns" (Math|Conversions|ToFloat(Integer) (.columns _value)) :!class /Script/Engine.MaterialInstanceDynamic)
      (bind _output_get (Variables|Default|SetFlipSprite (!= (Math|Conversions|ToBoolean(Integer) (Math|Integer|Clamp(Integer) (Math|Float|Truncate ActionValue) 0 1)) true)))
      (Rendering|Material|SetScalarParameterValue _charmat "FacingDir" (Math|Conversions|ToFloat(Boolean) _output_get) :!class /Script/Engine.MaterialInstanceDynamic)))
  (:Canceled
    (CallFunction|Idle :!label _label))
  (:Completed
    (goto _label)))

(event Input|EnhancedActionEvents|EnhancedInputActionIA_SplineJump
  (params (ActionValue :type Boolean) (ElapsedSeconds :type Float%20%28double-precision%29) (TriggeredSeconds :type Float%20%28double-precision%29) (InputAction :type Input%20Action%20Object%20Reference :default "/Game/Blueprints/Inputs/IA_SplineJump.IA_SplineJump"))
  (bind _returnvalue (Game|GetPlayerController 0))
  (bind _animationstatemappings (Variables|Default|GetAnimationStateMappings))
  (bind _charmat (Variables|Default|GetcharMat))
  (bind (_value _returnvalue_2) (Utilities|Map|Find _animationstatemappings "Jump"))
  (Input|DisableInput _returnvalue)
  (if _returnvalue_2
    (Rendering|Material|SetScalarParameterValue _charmat "UseAnimTimer" 1.0 :!class /Script/Engine.MaterialInstanceDynamic)
    (Rendering|Material|SetTextureParameterValue _charmat "Sprite" (.spritesheet _value))
    (Rendering|Material|SetScalarParameterValue _charmat "SpriteRows" (Math|Conversions|ToFloat(Integer) (.rows _value)) :!class /Script/Engine.MaterialInstanceDynamic)
    (Rendering|Material|SetScalarParameterValue _charmat "SpriteColumns" (Math|Conversions|ToFloat(Integer) (.columns _value)) :!class /Script/Engine.MaterialInstanceDynamic)
    (Character|Jump)
    (Variables|/Script/Engine.CharacterMovementComponent|SetbNotifyApex (Variables|Character|GetCharacterMovement) true)
    (Variables|Default|SetisJumping true)
    (Input|EnableInput _returnvalue)))

(event EventBeginPlay
  (Character|BindEventtoOnReachedJumpApex (delegate Custom|JumpApexReached)))

(event Collision|EventActorBeginOverlap
  (params (OtherActor :type Actor%20Object%20Reference)))

(event EventTick
  (params (DeltaSeconds :type Float%20%28single-precision%29))
  (if (not (Variables|Default|GetisJumping))
    (if (AI|Components|NavMovement|IsFalling (Variables|Character|GetCharacterMovement))
      (CallFunction|Falling))))

(event EventOnLanded
  (params (Hit :type Hit%20Result%20Structure%20%28by%20ref%29))
  (if (Variables|Default|GetisJumping)
    (Variables|Default|SetisJumping false))
  (CallFunction|Idle))

(fn ConstructionScript
  (bind _returnvalue (Rendering|Material|CreateDynamicMaterialInstance (Variables|Character|GetMesh) 0 "/Game/Materials/M_2_5D_Character.M_2_5D_Character" "None" :!class /Script/Engine.PrimitiveComponent))
  (bind _output_get (Variables|Default|SetcharMat _returnvalue))
  (Rendering|Material|SetMaterial (Variables|Character|GetMesh) 0 _output_get))